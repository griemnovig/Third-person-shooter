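; AI bot character Blueprint that manages a floating health bar above the bot.
; Health changes from STUHealthComponent are bound on BeginPlay to push the health percent into the WBP_BotHealthBar widget.
; A looping timer shows the bar only when the first player's controlled or spectator pawn is within a set distance, turning it toward that pawn as a manual billboard.
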(event `self.ReceiveBeginPlay`
  (`parent.ReceiveBeginPlay`)
  (add `STUHealthComponent.OnHealthChanged` (`self.STUHealthComponent`) (`|CreateDelegate` :!event `OnWidgetHealthChanged`))
  (`KismetSystemLibrary.K2_SetTimerDelegate` (`|CreateDelegate` :!event `UpdateHealthBarVisibility`) (`self.HealthBarUpdateVisibilityTime`) true))

(fn `OnWidgetHealthChanged`
  (params (Health :type "Float (single-precision)"))
  (bind _healthwidgetcomponent (`self.HealthWidgetComponent`)
    (:`then`
      (bind _aswbp_health_bar (cast `/Game/UI/WBP_BotHealthBar` (`WidgetComponent.GetUserWidgetObject` _healthwidgetcomponent)))
      (`/Game/UI/WBP_BotHealthBar.SetHealthPercent` _aswbp_health_bar (`STUHealthComponent.GetHealthPercent` (`self.STUHealthComponent`))))
    (:`else`)))

(fn `UpdateHealthBarVisibility`
  (locals (lPlayerPawn :type "Pawn Object Reference"))
  (bind _returnvalue (`GameplayStatics.GetPlayerController` 0))
  (bind _returnvalue_2 (`Controller.K2_GetPawn` _returnvalue))
  (`/Engine/EditorBlueprintResources/StandardMacros.IsValid` _returnvalue
    (:`Is Valid`
      (`/Engine/EditorBlueprintResources/StandardMacros.IsValid` _returnvalue_2
        (:`Is Valid`
          (set `local.lPlayerPawn` _returnvalue_2))
        (:`Is Not Valid`
          (set `local.lPlayerPawn` (`PlayerController.GetSpectatorPawn` (`GameplayStatics.GetPlayerController` 0)))))
      (bind _lplayerpawn (`local.lPlayerPawn`)
        (:`then`
          (if (< (`self.GetDistanceTo` _lplayerpawn) (`self.DistanceToHideHealthBar`))
            (`SceneComponent.SetVisibility` (`self.HealthWidgetComponent`) true true)
            (`SceneComponent.K2_SetWorldRotation` (`self.HealthWidgetComponent`) (`KismetMathLibrary.Conv_VectorToRotator` (`KismetMathLibrary.Normal` (- (`self.K2_GetActorLocation` (`local.lPlayerPawn`)) (`self.K2_GetActorLocation`)))) false true)
            (else
              (`SceneComponent.SetVisibility` (`self.HealthWidgetComponent`) false true :!label _label))))
        (:`else`
          (goto _label))))
    (:`Is Not Valid`
      (goto _label))))

(fn `UserConstructionScript`)