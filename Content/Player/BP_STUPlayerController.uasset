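; Player controller that sets up the HUD, input sensitivity and graphics settings when play begins.
; BeginPlay adds the general HUD, then applies saved pitch (negated) and yaw sensitivity and player name from the DefaultSlot save game.
; It also forces hardcoded scalability levels with VSync on and saves them.
; Holding Tab shows a freshly created players stat widget, removed on release.
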(event `self.ReceiveBeginPlay`
  (`parent.ReceiveBeginPlay`)
  (`|ExecutionSequence`
    (:`then_0`
      (bind _returnvalue (`|CreateWidget` "/Game/UI/WBP_GeneralHUD.WBP_GeneralHUD_C" self))
      (`UserWidget.AddToViewport` _returnvalue 0))
    (:`then_1`
      (`self.SetMouseSensitivity`)
      (bind _returnvalue_2 (`GameUserSettings.GetGameUserSettings`))
      (`GameUserSettings.SetVSyncEnabled` _returnvalue_2 true)
      (`GameUserSettings.SetAntiAliasingQuality` _returnvalue_2 2)
      (`GameUserSettings.SetShadowQuality` _returnvalue_2 3)
      (`GameUserSettings.SetViewDistanceQuality` _returnvalue_2 2)
      (`GameUserSettings.SetPostProcessingQuality` _returnvalue_2 0)
      (`GameUserSettings.SetGlobalIlluminationQuality` _returnvalue_2 2)
      (`GameUserSettings.SetReflectionQuality` _returnvalue_2 1)
      (`GameUserSettings.SetTextureQuality` _returnvalue_2 2)
      (`GameUserSettings.SetVisualEffectQuality` _returnvalue_2 1)
      (`GameUserSettings.SetFoliageQuality` _returnvalue_2 1)
      (`GameUserSettings.SetShadingQuality` _returnvalue_2 1)
      (`GameUserSettings.SaveSettings` _returnvalue_2))))

(event `Key|Tab`
  (params (Key :type "Key Structure"))
  (:`Pressed`
    (bind _returnvalue (`|CreateWidget` "/Game/UI/WBP_PlayersStat.WBP_PlayersStat_C" self))
    (`UserWidget.AddToViewport` _returnvalue 0))
  (:`Released`
    (`Widget.RemoveFromParent` _returnvalue)))

(fn `SetMouseSensitivity`
  (bind _returnvalue (`GameplayStatics.LoadGameFromSlot` "DefaultSlot"))
  (bind _asbp_save_game (cast `/Game/BP_SaveGame` _returnvalue))
  (`self.SetDeprecatedInputPitchScale` (* (`/Game/BP_SaveGame.GetMousePitchSensitivity` _asbp_save_game) -1.0))
  (`self.SetDeprecatedInputYawScale` (`/Game/BP_SaveGame.GetMouseYawSensitivity` _asbp_save_game))
  (`self.SetPlayerName` (`/Game/BP_SaveGame.GetPlayerName` _asbp_save_game)))

(fn `UserConstructionScript`)